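; WinLoseHalo is an actor that shows a Win or Lose component to mark the game's outcome.
; On BeginPlay it hides both components and caches the BP_Global actor.
; Each tick it polls that actor's IfWin and IfLose flags, reveals the matching component and slowly yaws the whole actor at a framerate-independent rate.
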(event `self.ReceiveBeginPlay`
  (bind _returnvalue (`GameplayStatics.GetActorOfClass` "/Game/Project/Blueprints/BP_Global.BP_Global_C"))
  (set `self.Global` _returnvalue)
  (`SceneComponent.SetVisibility` (`self.Win`) false false)
  (`SceneComponent.SetVisibility` (`self.Lose`) false false))

(event `self.ReceiveTick`
  (params (DeltaSeconds :type "Float (single-precision)"))
  (bind _returnvalue (`KismetMathLibrary.MakeRotator` 0.0 0.0 (* DeltaSeconds 10.0)))
  (`|ExecutionSequence`
    (:`then_0`
      (if (`/Game/Project/Blueprints/BP_Global.ifWin` (`self.Global`))
        (`SceneComponent.SetVisibility` (`self.Win`) true false)
        (`self.K2_AddActorWorldRotation` _returnvalue)))
    (:`then_1`
      (if (`/Game/Project/Blueprints/BP_Global.ifLose` (`self.Global`))
        (`SceneComponent.SetVisibility` (`self.Lose`) true false)
        (`self.K2_AddActorWorldRotation` _returnvalue)))))

(fn `UserConstructionScript`)