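; Global game manager actor that runs asteroid spawning, pause, win/lose checks and level progression around the planet's population.
; A looping timer, its interval derived from Level at BeginPlay, spawns asteroids around the planet, rerolling random positions until they fall within a sun-facing cone.
; Tick halts play and planet rotation when population hits zero or the maximum.
; NextLevel fades the camera, resets population and asteroids, and increments Level after a win.
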(event `self.ReceiveBeginPlay`
  (`|ExecutionSequence`
    (:`then_0`
      (bind _returnvalue (`GameplayStatics.GetActorOfClass` "/Game/Project/Blueprints/BP_Sun.BP_Sun_C"))
      (set `self.sun_dir` (`KismetMathLibrary.Normal` (`self.K2_GetActorLocation` _returnvalue))))
    (:`then_1`
      ;[1 1 1] Spawn Asteriods
      (`KismetSystemLibrary.K2_SetTimerDelegate` (delegate `Event Spawn`) (`KismetMathLibrary.Conv_IntToDouble` (`KismetMathLibrary.Clamp` (- 5 (`self.level`)) 1 5)) true))
    (:`then_2`
      (`|ExecutionSequence`
        (:`then_2`
          (bind _returnvalue_2 (`|CreateWidget` "/Game/Project/Blueprints/WinScreen.WinScreen_C"))
          (bind _output_get (set `self.Win` _returnvalue_2))
          (`UserWidget.AddToViewport` _output_get 0)
          (`Widget.SetVisibility` (`self.Win`) "Hidden"))
        (:`then_3`
          (bind _returnvalue_3 (`|CreateWidget` "/Game/Project/Blueprints/LoseScreen.LoseScreen_C"))
          (bind _output_get_2 (set `self.Lose` _returnvalue_3))
          (`UserWidget.AddToViewport` _output_get_2 0)
          (`Widget.SetVisibility` (`self.Lose`) "Hidden"))))
    (:`then_3`
      (bind _returnvalue_4 (`GameplayStatics.GetActorOfClass` "/Game/Project/Blueprints/BP_Planet.BP_Planet_C"))
      (set `self.Planet` _returnvalue_4))
    (:`then_4`
      (`AudioComponent.Play` (`self.background`) 0.0))))

(event `Event Spawn`
  (if (not (`self.Paused`))
    ;[1 1 1] Spawn Asteriods
    (`|ExecutionSequence`
      (:`then_0`
        (`self.GetValidSpawnPosition`))
      (:`then_1`
        (`|SpawnActorFromClass` "/Game/Project/Blueprints/BP_Astroid.BP_Astroid_C" (`KismetMathLibrary.Conv_VectorToTransform` (`self.spawnPos`)) "Undefined" "OverrideRootScale" null null)))))

(event `self.ReceiveTick`
  (params (DeltaSeconds :type "Float (single-precision)"))
  (`self.Winning Condition`))

(event `PauseOrResume`
  ;[1 1 1] Pause
  (`/Engine/EditorBlueprintResources/StandardMacros.FlipFlop`
    (:`A`
      (set `self.Paused` true))
    (:`B`
      (set `self.Paused` false))))

(event `Winning Condition`
  (bind _population (`/Game/Project/Blueprints/BP_Planet.Population` (`self.Planet`)))
  ;[1 1 1] Win or Lose
  (`|ExecutionSequence`
    (:`then_0`
      (if (>= _population (`self.MaxPopulation`))
        (`Widget.SetVisibility` (`self.Win`) "Hidden")
        (set `self.Paused` true)
        (set `self.ifWin` true)
        (set `/Game/Project/Blueprints/BP_Planet.RotRate` 0.0 (`self.Planet`) :!label _label)))
    (:`then_1`
      (if (<= _population 0.0)
        (`Widget.SetVisibility` (`self.Lose`) "Hidden")
        (set `self.Paused` true)
        (set `self.ifLose` true)
        (goto _label)))))

(event `NextLevel`
  ;[1 1 1] Update Level
  (`PlayerCameraManager.StartCameraFade` :`self` (`GameplayStatics.GetPlayerCameraManager` 0) :`ToAlpha` 1.0 :`Duration` 0.5 :`bHoldWhenFinished` true)
  (if (`self.ifWin`)
    (set `self.level` (+ (`self.level`) 1)))
  (set `/Game/Project/Blueprints/BP_Planet.Population` 50.0 (`self.Planet`))
  (bind _outactors (`GameplayStatics.GetAllActorsOfClass` "/Game/Project/Blueprints/BP_Astroid.BP_Astroid_C"))
  (for _array_element _outactors
    (`self.K2_DestroyActor` _array_element))
  (`Widget.SetVisibility` (`self.Lose`) "Hidden")
  (`Widget.SetVisibility` (`self.Win`) "Hidden")
  (set `self.ifWin` false)
  (set `self.ifLose` false)
  (set `self.Paused` false)
  (`PlayerCameraManager.StartCameraFade` :`self` (`GameplayStatics.GetPlayerCameraManager` 0) :`FromAlpha` 1.0 :`Duration` 0.8 :`bHoldWhenFinished` true))

(fn `UserConstructionScript`)