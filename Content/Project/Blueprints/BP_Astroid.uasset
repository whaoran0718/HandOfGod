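; BP_Astroid is an asteroid actor that falls toward the world origin and reduces the planet's population on impact.
; BeginPlay sets a constant inward velocity and caches BP_Planet and BP_Global; Tick moves it without sweep unless Global's tickable-when-paused flag is set.
; Each moving tick, BeHit queries Planet.ShowLaunchPlane; within the planet radius, it subtracts that result times DeathRate from Population and destroys itself.
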(event `self.ReceiveBeginPlay`
  (`|ExecutionSequence`
    (:`then_0`
      (set `self.velocity` (* (`KismetMathLibrary.Normal` (`SceneComponent.K2_GetComponentLocation` (`self.collider`))) -30.0)))
    (:`then_1`
      (bind _returnvalue (`GameplayStatics.GetActorOfClass` "/Game/Project/Blueprints/BP_Planet.BP_Planet_C"))
      (set `self.planet` _returnvalue))
    (:`then_2`
      (bind _returnvalue_2 (`GameplayStatics.GetActorOfClass` "/Game/Project/Blueprints/BP_Global.BP_Global_C"))
      (set `self.global` _returnvalue_2))))

(event `self.ReceiveTick`
  (params (DeltaSeconds :type "Float (single-precision)"))
  (bind _returnvalue (`self.GetTickableWhenPaused` (`self.global`)))
  (if (not _returnvalue)
    (`|ExecutionSequence`
      (:`then_0`
        (`self.K2_AddActorWorldOffset` (* (`self.velocity`) DeltaSeconds)))
      (:`then_1`
        (`self.BeHit`)))))

(event `BeHit`
  (bind _planet (`self.planet`))
  (bind _returnvalue (`Planet.ShowLaunchPlane` (`self.planet`) (`SceneComponent.K2_GetComponentLocation` (`self.AsteroidMesh`)) 10.0))
  (if (<= (`KismetMathLibrary.VSize` (`SceneComponent.K2_GetComponentLocation` (`self.AsteroidMesh`))) (`Planet.Radius` (`self.planet`)))
    (`KismetSystemLibrary.PrintString` "destroy population" true true (struct :`R` 1.0 :`G` 0.019096 :`A` 1.0))
    (set `/Game/Project/Blueprints/BP_Planet.Population` (- (`/Game/Project/Blueprints/BP_Planet.Population` _planet) (* _returnvalue (`self.DeathRate`))) _planet)
    (`self.K2_DestroyActor`)))

(fn `GetEarthLocation`
  (bind _returnvalue (`GameplayStatics.GetActorOfClass` null))
  (set `self.EarthLocation` (`self.K2_GetActorLocation` _returnvalue)))

(fn `UserConstructionScript`)